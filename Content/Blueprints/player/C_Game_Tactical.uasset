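; Player-controlled free-fly camera character or pawn for the game's tactical view.
; Enhanced Input actions drive look, fly, strafe, ascent and pan through controller rotation and actor-relative movement input.
; A ToggleMouseCursor macro hides the cursor on the cached PC_Game_Tactical while looking or panning.
; Clicks trace under the cursor on Visibility and send OnGameObjectClickedMessage to the hit actor; Focus is a stub.
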(event `self.ReceiveBeginPlay`
  (bind _aspc_game_tactical (cast `/Game/Blueprints/player/PC_Game_Tactical` (`self.GetController`)))
  (set `self.PlayerController` _aspc_game_tactical))

(event `EnhancedInput|/Game/Controls/Tactical_Look`
  (params (ActionValue :type Boolean) (ElapsedSeconds :type "Float (double-precision)") (TriggeredSeconds :type "Float (double-precision)") (InputAction :type "InputAction Object Reference" :default "/Game/Controls/Tactical_Look.Tactical_Look"))
  (bind _lookspeed (`self.LookSpeed`))
  (:`Triggered`
    (`self.AddControllerPitchInput` (* (* (`self.GetInputAxisKeyValue`) _lookspeed) -1.0))
    (`self.AddControllerYawInput` (* _lookspeed (`self.GetInputAxisKeyValue`))))
  (:`Started`
    (`self.ToggleMouseCursor` :!label _label))
  (:`Canceled`
    (goto _label :!via `Show Mouse Cursor`))
  (:`Completed`
    (goto _label :!via `Show Mouse Cursor`)))

(event `EnhancedInput|/Game/Controls/Tactical_Fly`
  (params (ActionValue :type "Float (double-precision)") (ElapsedSeconds :type "Float (double-precision)") (TriggeredSeconds :type "Float (double-precision)") (InputAction :type "InputAction Object Reference" :default "/Game/Controls/Tactical_Fly.Tactical_Fly"))
  (:`Triggered`
    (`self.AddMovementInput` (`self.GetActorForwardVector`) (* ActionValue (`self.FlySpeed`)))))

(event `EnhancedInput|/Game/Controls/Tactical_Strafe`
  (params (ActionValue :type "Float (double-precision)") (ElapsedSeconds :type "Float (double-precision)") (TriggeredSeconds :type "Float (double-precision)") (InputAction :type "InputAction Object Reference" :default "/Game/Controls/Tactical_Strafe.Tactical_Strafe"))
  (:`Triggered`
    (`self.AddMovementInput` (`self.GetActorRightVector`) (* ActionValue (`self.FlySpeed`)))))

(event `EnhancedInput|/Game/Controls/Tactical_Ascent`
  (params (ActionValue :type "Float (double-precision)") (ElapsedSeconds :type "Float (double-precision)") (TriggeredSeconds :type "Float (double-precision)") (InputAction :type "InputAction Object Reference" :default "/Game/Controls/Tactical_Ascent.Tactical_Ascent"))
  (:`Triggered`
    (`self.AddMovementInput` (`self.GetActorUpVector`) (* ActionValue (`self.FlySpeed`)))))

(event `EnhancedInput|/Game/Controls/Tactical_Pan`
  (params (ActionValue :type Boolean) (ElapsedSeconds :type "Float (double-precision)") (TriggeredSeconds :type "Float (double-precision)") (InputAction :type "InputAction Object Reference" :default "/Game/Controls/Tactical_Pan.Tactical_Pan"))
  (:`Triggered`
    (`self.AddMovementInput` (+ (* (`self.GetActorRightVector`) (`self.GetInputAxisKeyValue`)) (* (`self.GetActorUpVector`) (`self.GetInputAxisKeyValue`))) (`self.PanSpeed`)))
  (:`Started`
    (`self.ToggleMouseCursor` :!label _label_2))
  (:`Canceled`
    (goto _label_2 :!via `Show Mouse Cursor`))
  (:`Completed`
    (goto _label_2 :!via `Show Mouse Cursor`)))

(event `EnhancedInput|/Game/Controls/Tactical_Click`
  (params (ActionValue :type Boolean) (ElapsedSeconds :type "Float (double-precision)") (TriggeredSeconds :type "Float (double-precision)") (InputAction :type "InputAction Object Reference" :default "/Game/Controls/Tactical_Click.Tactical_Click"))
  (:`Triggered`
    (message `/Game/Blueprints/coding/I_Tactical.OnGameObjectClicked` (`.HitActor` (`GameplayStatics.BreakHitResult` (`PlayerController.GetHitResultUnderCursorByChannel` (`self.PlayerController`) "TraceTypeQuery1" true))))))

(event `EnhancedInput|/Game/Controls/Tactical_Focus`
  (params (ActionValue :type "Float (double-precision)") (ElapsedSeconds :type "Float (double-precision)") (TriggeredSeconds :type "Float (double-precision)") (InputAction :type "InputAction Object Reference" :default "/Game/Controls/Tactical_Focus.Tactical_Focus"))
  (:`Completed`
    (`KismetSystemLibrary.PrintString` "\"Tactical Focus\" not implemented...")))

(fn `UserConstructionScript`)