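; AC_GameplayTagsManager is an actor component that holds a gameplay tag container for its owning actor.
; Events add or remove tags in that container.
; Functions check whether a tag is present, with optional exact matching, or return the whole container.
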(event `/Game/Blueprints/coding/I_GameplayTags.AddGameplayTagToActor`
  (params (NewGameplayTag :type "GameplayTag Structure"))
  (`BlueprintGameplayTagLibrary.AddGameplayTag` (`self.GameplayTags`) NewGameplayTag))

(event `/Game/Blueprints/coding/I_GameplayTags.RemoveGameplayTagFromActor`
  (params (GameplayTagToBeRemoved :type "GameplayTag Structure"))
  (`BlueprintGameplayTagLibrary.RemoveGameplayTag` (`self.GameplayTags`) GameplayTagToBeRemoved))

(fn `CheckForTagOnTarget`
  (params (tag :type "GameplayTag Structure") (exact :type Boolean))
  (returns (result :type Boolean))
  (return (`BlueprintGameplayTagLibrary.HasTag` (`self.GameplayTags`) tag exact)))

(fn `GetTagsOnTarget`
  (returns (TargetTags :type "GameplayTagContainer Structure"))
  (return (`self.GameplayTags`)))