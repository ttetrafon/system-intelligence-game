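; Game instance that holds and persists the player's game settings (visual quality and mouse sensitivity) across sessions.
; LoadSettings reads the SD_GameSettings save slot into GameSettings, or writes the current values to a new save if none exists.
; Update events change a single field only when its value differs, then SaveGameSettings writes a fresh save object to the slot.
; It only stores these values; applying them is not done here.
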(event `/Game/Blueprints/I_Settings.LoadSettings`
  (bind _savegameslot_settings (`self.SaveGameSlot_Settings`))
  (bind _returnvalue (`GameplayStatics.DoesSaveGameExist` _savegameslot_settings))
  (if _returnvalue
    (bind _returnvalue_2 (`GameplayStatics.LoadGameFromSlot` _savegameslot_settings))
    (bind _assd_game_settings (cast `/Game/Data/SD_GameSettings` _returnvalue_2)
      (:`then`
        (set `self.GameSettings` (`/Game/Data/SD_GameSettings.GameSettings` _assd_game_settings))
        (`KismetSystemLibrary.PrintString` "Loaded settings!"))
      (:`CastFailed`
        (`KismetSystemLibrary.PrintString` "failed to cast...")))
    (else
      (`self.SaveGameSettings` (`self.GameSettings`))
      (`KismetSystemLibrary.PrintString` "Loading settings faild, had to create the save-file!"))))

(event `/Game/Blueprints/I_Settings.VisualQualityUpdate`
  (params (VisualQuality :type Integer))
  (bind (_gamesettings_visualquality _gamesettings_mousesensitivity) (break `/Game/Data/S_GameSettings` (`self.GameSettings`)))
  (if (!= VisualQuality _gamesettings_visualquality)
    (bind _output_get (set `self.GameSettings` (make `/Game/Data/S_GameSettings` VisualQuality _gamesettings_mousesensitivity)))
    (`self.SaveGameSettings` _output_get)))

(event `/Game/Blueprints/I_Settings.MouseSensitivityUpdate`
  (params (MouseSensitivity :type "Float (double-precision)"))
  (bind (_gamesettings_visualquality _gamesettings_mousesensitivity) (break `/Game/Data/S_GameSettings` (`self.GameSettings`)))
  (if (!= MouseSensitivity _gamesettings_mousesensitivity)
    (bind _output_get (set `self.GameSettings` (make `/Game/Data/S_GameSettings` _gamesettings_visualquality MouseSensitivity)))
    (`self.SaveGameSettings` _output_get)))

(fn `SaveGameSettings`
  (params (GameSettings :type "/Game/Data/S_GameSettings Structure"))
  (bind _returnvalue (`GameplayStatics.CreateSaveGameObject` "/Game/Data/SD_GameSettings.SD_GameSettings_C"))
  (set `/Game/Data/SD_GameSettings.GameSettings` GameSettings _returnvalue)
  (`GameplayStatics.SaveGameToSlot` _returnvalue (`self.SaveGameSlot_Settings`)))