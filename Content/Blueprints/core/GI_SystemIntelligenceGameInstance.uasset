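; Game instance that loads, validates and persists player settings: name, mouse sensitivity and visual quality.
; On Init it loads the settings save slot, or saves the current defaults if none exists.
; Update events change one field and write a new SD_GameSettings save object only when the value differs.
; A consistency check on loaded settings gives an empty player name a random "Player-" numbered name.
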(event `self.ReceiveInit`
  (bind _savegameslot_settings (`self.SaveGameSlot_Settings`))
  (bind _returnvalue (`GameplayStatics.DoesSaveGameExist` _savegameslot_settings))
  (if _returnvalue
    (bind _returnvalue_2 (`GameplayStatics.LoadGameFromSlot` _savegameslot_settings))
    (bind _assd_game_settings (cast `/Game/Data/SD_GameSettings` _returnvalue_2))
    (bind _output_get (set `self.GameSettings` (`/Game/Data/SD_GameSettings.GameSettings` _assd_game_settings)))
    (`self.CheckSettingsForConsistency` _output_get)
    (else
      (`self.SaveGameSettings` (`self.GameSettings`)))))

(event `/Game/Blueprints/coding/I_Settings.VisualQualityUpdate`
  (params (VisualQuality :type Integer))
  (bind (_gamesettings_playername _gamesettings_mousesensitivity _gamesettings_visualquality) (break `/Game/Data/S_GameSettings` (`self.GameSettings`)))
  ;[1 1 1] Settings
  (if (!= VisualQuality _gamesettings_visualquality)
    (bind _output_get (set `self.GameSettings` (make `/Game/Data/S_GameSettings` _gamesettings_playername _gamesettings_mousesensitivity VisualQuality)))
    (`self.SaveGameSettings` _output_get)))

(event `/Game/Blueprints/coding/I_Settings.MouseSensitivityUpdate`
  (params (MouseSensitivity :type "Float (double-precision)"))
  (bind (_gamesettings_playername _gamesettings_mousesensitivity _gamesettings_visualquality) (break `/Game/Data/S_GameSettings` (`self.GameSettings`)))
  ;[1 1 1] Settings
  (if (!= MouseSensitivity _gamesettings_mousesensitivity)
    (bind _output_get (set `self.GameSettings` (make `/Game/Data/S_GameSettings` _gamesettings_playername MouseSensitivity _gamesettings_visualquality)))
    (`self.SaveGameSettings` _output_get)))

(event `/Game/Blueprints/coding/I_Settings.PlayerNameUpdate`
  (params (PlayerName :type String))
  (bind (_gamesettings_playername _gamesettings_mousesensitivity _gamesettings_visualquality) (break `/Game/Data/S_GameSettings` (`self.GameSettings`)))
  ;[1 1 1] Settings
  (if (`KismetStringLibrary.NotEqual_StrStr` PlayerName _gamesettings_playername)
    (bind _output_get (set `self.GameSettings` (make `/Game/Data/S_GameSettings` PlayerName _gamesettings_mousesensitivity _gamesettings_visualquality)))
    (`self.SaveGameSettings` _output_get)))

(fn `SaveGameSettings`
  (params (GameSettings :type "/Game/Data/S_GameSettings Structure"))
  (bind _returnvalue (`GameplayStatics.CreateSaveGameObject` "/Game/Data/SD_GameSettings.SD_GameSettings_C"))
  (set `/Game/Data/SD_GameSettings.GameSettings` GameSettings _returnvalue)
  (`GameplayStatics.SaveGameToSlot` _returnvalue (`self.SaveGameSlot_Settings`)))