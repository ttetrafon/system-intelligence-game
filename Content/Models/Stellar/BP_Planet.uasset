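; BP_Planet is a planet actor that orbits a centre actor at a set speed, with its material applied in the construction script.
; Each tick it rotates its offset from the previous centre around the orbit axis, then adds the current centre so the orbit follows a moving target.
; Before each step, a double cross product makes the axis perpendicular to that offset and normalises it.
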(event `self.ReceiveBeginPlay`
  (`|ExecutionSequence`
    (:`then_0`
      (bind _centeactor (`self.CenteActor`)
        (:`then`
          (set `self.CentreLocation` (`self.K2_GetActorLocation` _centeactor)))
        (:`else`)))
    (:`then_1`
      (set `self.OldCentreLocation` (`self.CentreLocation`)))))

(event `self.ReceiveTick`
  (params (DeltaSeconds :type "Float (single-precision)"))
  (`|ExecutionSequence`
    (:`then_0`
      (bind _centeactor (`self.CenteActor`)
        (:`then`
          (set `self.CentreLocation` (`self.K2_GetActorLocation` _centeactor)))
        (:`else`)))
    (:`then_1`
      (`self.OrthogonaliseAxis`)
      (`self.K2_SetActorLocation` (+ (`KismetMathLibrary.RotateAngleAxis` (- (`self.K2_GetActorLocation`) (`self.OldCentreLocation`)) (* DeltaSeconds (`self.Speed`)) (`self.AxisOfRotation`)) (`self.CentreLocation`)))
      (set `self.OldCentreLocation` (`self.CentreLocation`)))))

(event `OrthogonaliseAxis`
  (bind _returnvalue (- (`self.K2_GetActorLocation`) (`self.OldCentreLocation`)))
  (set `self.AxisOfRotation` (`KismetMathLibrary.Normal` (`KismetMathLibrary.Cross_VectorVector` _returnvalue (`KismetMathLibrary.Cross_VectorVector` (`self.AxisOfRotation`) _returnvalue)))))

(fn `UserConstructionScript`
  (`PrimitiveComponent.SetMaterial` (`self.mesh`) 0 (`self.Material`)))